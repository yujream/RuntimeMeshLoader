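; Actor Blueprint that imports a mesh from a file path at runtime and builds it as procedural geometry.
; On BeginPlay it loads the file asynchronously and, on success, loops over the returned mesh infos.
; Each entry gets its own ProceduralMeshComponent at its relative transform, with a collision-enabled section.
; The entry's array index sets both the section index and the slot picked from the Material array.
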(event EventBeginPlay
  (bind _result (|LoadMeshAsync (Variables|Default|GetFilePath) (Variables|Default|GetPathType))
    (:OnComplete
      (if (.bSuccess (Utilities|Struct|BreakReturnedData _result))
        (for (_array_element _array_index) (.meshInfo (Utilities|Struct|BreakReturnedData _result))
          (bind _returnvalue (AddComponent|AddProceduralMeshComponent false (.RelativeTransform (Utilities|Struct|BreakModelMeshInfo _array_element))))
          (Class|ProceduralMeshComponent|CreateMeshSectionLinearColor _returnvalue _array_index (.Vertices (Utilities|Struct|BreakModelMeshInfo _array_element)) (.Triangles (Utilities|Struct|BreakModelMeshInfo _array_element)) (.Normals (Utilities|Struct|BreakModelMeshInfo _array_element)) (.UV0 (Utilities|Struct|BreakModelMeshInfo _array_element)) 0 0 0 (.VertexColors (Utilities|Struct|BreakModelMeshInfo _array_element)) (.Tangents (Utilities|Struct|BreakModelMeshInfo _array_element)) true false)
          (Rendering|Material|SetMaterial _returnvalue _array_index (Utilities|Array|Get(acopy) (Variables|Default|GetMaterial) _array_index)))))))

(fn ConstructionScript)